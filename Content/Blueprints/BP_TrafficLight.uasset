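; BP_TrafficLight is a traffic light that signals passing cars to stop or go.
; Started and Stoped re-schedule each other by timer every four seconds, swapping materials on two cubes and flipping the Stop flag.
; Each Tick runs short world +X line traces from four arrows, caching the hit actor.
; A hit calls stop or start per the flag: Car1 variants for the first arrow, generic ones for the rest.
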(event EventBeginPlay
  (CallFunction|Started))

(event Collision|EventActorBeginOverlap
  (params (OtherActor :type Actor%20Object%20Reference)))

(event EventTick
  (params (DeltaSeconds :type Float%20%28single-precision%29))
  (bind _arrow (Variables|Default|GetArrow))
  (bind _arrow1 (Variables|Default|GetArrow1))
  (bind _arrow2 (Variables|Default|GetArrow2))
  (bind _arrow3 (Variables|Default|GetArrow3))
  (bind _returnvalue (Transformation|GetWorldLocation _arrow3))
  (bind _returnvalue_2 (Transformation|GetWorldLocation _arrow2))
  (bind _returnvalue_3 (Transformation|GetWorldLocation _arrow))
  (bind _returnvalue_4 (Transformation|GetWorldLocation _arrow1))
  ;[1 1 1] Проверка на присутствие машины
  (Utilities|FlowControl|Sequence
    (:then_0
      (bind (_outhit _returnvalue_5) (Collision|LineTraceByChannel (Math|Vector|MakeVector (.x _returnvalue_3) (.y _returnvalue_3) (.z _returnvalue_3)) (Math|Vector|MakeVector (+ (.x _returnvalue_3) 1e+01) (.y _returnvalue_3) (.z _returnvalue_3)) "TraceTypeQuery1" false 0 "None"))
      (if _returnvalue_5
        (Variables|Default|SetHit%20Actor (.HitActor (Collision|BreakHitResult _outhit)))
        (Variables|Default|SetHit%20Actor_0 0)
        (if (Variables|Default|Get?Stop)
          (Default|CallStopCar1)
          (else
            (Default|CallStartCar1)))))
    (:then_1
      (bind (_outhit_2 _returnvalue_6) (Collision|LineTraceByChannel (Math|Vector|MakeVector (.x _returnvalue_4) (.y _returnvalue_4) (.z _returnvalue_4)) (Math|Vector|MakeVector (+ (.x _returnvalue_4) 1e+01) (.y _returnvalue_4) (.z _returnvalue_4)) "TraceTypeQuery1" false 0 "None"))
      (if _returnvalue_6
        (Variables|Default|SetHit%20Actor_0 (.HitActor (Collision|BreakHitResult _outhit_2)))
        (Variables|Default|SetHit%20Actor 0)
        (if (Variables|Default|Get?Stop)
          (Default|CallStop)
          (else
            (Default|CallStart)))))
    (:then_2
      (bind (_outhit_3 _returnvalue_7) (Collision|LineTraceByChannel (Math|Vector|MakeVector (.x _returnvalue_2) (.y _returnvalue_2) (.z _returnvalue_2)) (Math|Vector|MakeVector (+ (.x _returnvalue_2) 1e+01) (.y _returnvalue_2) (.z _returnvalue_2)) "TraceTypeQuery1" false 0 "None"))
      (if _returnvalue_7
        (Variables|Default|SetHit%20Actor_0 (.HitActor (Collision|BreakHitResult _outhit_3)))
        (Variables|Default|SetHit%20Actor 0)
        (if (Variables|Default|Get?Stop)
          (Default|CallStop)
          (else
            (Default|CallStart)))))
    (:then_3
      (bind (_outhit_4 _returnvalue_8) (Collision|LineTraceByChannel (Math|Vector|MakeVector (.x _returnvalue) (.y _returnvalue) (.z _returnvalue)) (Math|Vector|MakeVector (+ (.x _returnvalue) 1e+01) (.y _returnvalue) (.z _returnvalue)) "TraceTypeQuery1" false 0 "None"))
      (if _returnvalue_8
        (Variables|Default|SetHit%20Actor_0 (.HitActor (Collision|BreakHitResult _outhit_4)))
        (Variables|Default|SetHit%20Actor 0)
        (if (Variables|Default|Get?Stop)
          (Default|CallStop)
          (else
            (Default|CallStart)))))))

(fn ConstructionScript)

(fn Stoped
  (Utilities|Time|SetTimerbyFunctionName 0 "Started" 4.0)
  (Rendering|Material|SetMaterial (Variables|Default|GetCube3) 0 "/Game/ModularBuildingSet/materials/Bricks_Tiles/brick_wall_dark_red.brick_wall_dark_red")
  (Rendering|Material|SetMaterial (Variables|Default|GetCube2) 0 "/Engine/BasicShapes/BasicShapeMaterial.BasicShapeMaterial")
  (Variables|Default|Set?Stop true))

(fn Started
  (Utilities|Time|SetTimerbyFunctionName 0 "Stoped" 4.0)
  (Rendering|Material|SetMaterial (Variables|Default|GetCube2) 0 "/Game/ModularBuildingSet/materials/Bricks_Tiles/brick_wall_dark_red.brick_wall_dark_red")
  (Rendering|Material|SetMaterial (Variables|Default|GetCube3) 0 "/Engine/BasicShapes/BasicShapeMaterial.BasicShapeMaterial")
  (Variables|Default|Set?Stop false))