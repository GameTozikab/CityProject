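; BP_Cars spawns a random car class and drives it along a spline, respawning another when it finishes.
; A timeline feeds MoveCar, which sets the car's transform from the spline at that time.
; On each timeline update it checks every BP_TrafficLight, binding start/stop events where the car matches HitActor or HitActor0 to play or stop the timeline.
; The HitActor binding inverts that mapping, and an alternative collapsed spawn graph never runs.
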(event EventBeginPlay
  (bind _class (Variables|Default|GetClass))
  ;[1 1 1] Выбор рандомной машины
  (bind _returnvalue (Game|SpawnActorfromClass (Utilities|Array|Get(acopy) _class (Math|Random|RandomInteger (Utilities|Array|Length _class))) (Transformation|GetWorldTransform (Variables|Default|GetSpline)) "Undefined" 0 0 :!label _label))
  (Utilities|IsValid _returnvalue
    (:Is%20Valid
      (if (Variables|Default|GetNewVar_1)
        (bind _newtrack_0 (Timeline|Timeline_1 Play)
          (:Update
            (CallFunction|MoveCar _newtrack_0 _returnvalue)
            (Utilities|FlowControl|Sequence
              (:then_0
                ;[1 1 1] Указание действия машине
                (bind _outactors (Actor|GetAllActorsOfClass "/Game/Blueprints/BP_TrafficLight.BP_TrafficLight_C"))
                (for (_array_element _array_index) _outactors
                  (|CollapseGraph_0_2 _array_element _array_index _returnvalue
                    (:start
                      (Timeline|Timeline_1 Stop))
                    (:stop
                      (Timeline|Timeline_1 Play)))))
              (:then_1
                (bind _outactors_2 (Actor|GetAllActorsOfClass "/Game/Blueprints/BP_TrafficLight.BP_TrafficLight_C"))
                (for (_array_element_2 _array_index_2) _outactors_2
                  (|CollapseGraph_0 _array_element_2 _array_index_2 _returnvalue
                    (:start
                      (Timeline|Timeline_1 Play))
                    (:stop
                      (Timeline|Timeline_1 Stop)))))))
          (:Finished
            ;[1 1 1] удаление машины при достижении цели
            (Actor|DestroyActor _returnvalue)
            (Utilities|FlowControl|Delay 0.2)
            (Variables|Default|SetNewVar_1 false)
            (goto _label)))
        (else
          (Timeline|Timeline_1 PlayFromStart))))))

(event Collision|EventActorBeginOverlap
  (params (OtherActor :type Actor%20Object%20Reference)))

(event EventTick
  (params (DeltaSeconds :type Float%20%28single-precision%29)))

(fn ConstructionScript)

(fn MoveCar
  (params (Time :type Float%20%28single-precision%29) (self2 :type Actor%20Object%20Reference))
  (Utilities|IsValid self2
    (:Is%20Valid
      (Transformation|SetActorRelativeTransform self2 (Spline|GetTransformatTime (Variables|Default|GetSpline) Time "World" false false) false false))))

(event Custom|StartCar1_Event_0
  (return))

(event Custom|StopCar1_Event_0
  (return))

(event Custom|Stop_Event_0
  (bind _newtrack_0 (Timeline|Timeline_0 Stop)
    (:Update
      (CallFunction|MoveCar _newtrack_0 (stale _returnvalue)))
    (:Finished
      (Actor|DestroyActor (stale _returnvalue))
      (Utilities|FlowControl|Delay 0.2)
      (Variables|Default|SetNewVar_1 false)
      (bind _returnvalue (Game|SpawnActorfromClass (Utilities|Array|Get(acopy) (Variables|Default|GetClass) (Variables|Default|GetN_Car)) (Transformation|GetWorldTransform (Variables|Default|GetSpline)) "Undefined" 0 (Game|GetInstigator)))
      (Utilities|IsValid _returnvalue
        (:Is%20Valid
          (if (Variables|Default|GetNewVar_1)
            (Timeline|Timeline_0 Play)
            (else
              (Timeline|Timeline_0 PlayFromStart))))))))

(event Custom|Start_Event_0
  (bind _newtrack_0 (Timeline|Timeline_0 Play)
    (:Update
      (CallFunction|MoveCar _newtrack_0 (stale _returnvalue)))
    (:Finished
      (Actor|DestroyActor (stale _returnvalue))
      (Utilities|FlowControl|Delay 0.2)
      (Variables|Default|SetNewVar_1 false)
      (bind _returnvalue (Game|SpawnActorfromClass (Utilities|Array|Get(acopy) (Variables|Default|GetClass) (Variables|Default|GetN_Car)) (Transformation|GetWorldTransform (Variables|Default|GetSpline)) "Undefined" 0 (Game|GetInstigator)))
      (Utilities|IsValid _returnvalue
        (:Is%20Valid
          (if (Variables|Default|GetNewVar_1)
            (Timeline|Timeline_0 Play)
            (else
              (Timeline|Timeline_0 PlayFromStart))))))))

(event Custom|Start_Event_2
  (|Outputs) ; enters at start
)

(event Custom|Stop_Event_2
  (|Outputs) ; enters at stop
)